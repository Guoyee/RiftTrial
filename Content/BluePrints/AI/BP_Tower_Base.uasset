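; Base Blueprint for an AI tower that repeatedly tries to use its Gameplay Ability System abilities.
; On BeginPlay it caches its Ability System Component and, if valid, starts a short looping timer with a stored handle.
; Each tick of the timer tries to activate abilities matching the GameplayTags array, without acting on the result.
; It contains no targeting logic of its own.
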(event `self.ReceiveBeginPlay`
  (bind _output_get (set `self.ASC` (`AbilitySystemBlueprintLibrary.GetAbilitySystemComponent` null)))
  (if (`KismetSystemLibrary.IsValid` _output_get)
    (bind _returnvalue (`KismetSystemLibrary.K2_SetTimerDelegate` (delegate `AttemptActivateAbility`) 0.2 true))
    (set `self.AbilityTimerHandle` _returnvalue)))

(event `AttemptActivateAbility`
  (bind _returnvalue (`AbilitySystemComponent.TryActivateAbilitiesByTag` (`self.ASC`) (`BlueprintGameplayTagLibrary.MakeGameplayTagContainerFromArray` (`self.Gameplay Tags`)) true))
  (if _returnvalue
    _))

(fn `UserConstructionScript`)